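; Game mode for a robot arena match that spawns three test robots and one dummy robot at BeginPlay.
; RandomTransform gives each a random floor position and yaw within the arena bounds, and the robots are tracked in RobotAlive.
; Each robot gets a color by array index, plus a main widget added to the viewport with UI-only input.
; RandomiseRobot re-rolls placement but returns inside its loop, so only the first robot moves.
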(event `self.ReceiveBeginPlay`
  (bind _robotalive (`self.RobotAlive`))
  ;[1 1 1] Spawning Robot 1
  (bind _randomtransform (`self.Random Transform`))
  (bind _returnvalue (`|SpawnActorFromClass` "/Game/Blueprint/RobotTest_BP.RobotTest_BP_C" _randomtransform "Undefined" "OverrideRootScale" null null))
  (`KismetArrayLibrary.Array_Add` _robotalive _returnvalue)
  ;[1 1 1] Spawning robot 2
  (bind _randomtransform_2 (`self.Random Transform`))
  (bind _returnvalue_2 (`|SpawnActorFromClass` "/Game/Blueprint/DummyRobot_BP.DummyRobot_BP_C" _randomtransform_2 "Undefined" "OverrideRootScale" null null))
  (`KismetArrayLibrary.Array_Add` _robotalive _returnvalue_2)
  ;[1 1 1] Spawning Robot 3
  (bind _randomtransform_3 (`self.Random Transform`))
  (bind _returnvalue_3 (`|SpawnActorFromClass` "/Game/Blueprint/RobotTest_BP.RobotTest_BP_C" _randomtransform_3 "Undefined" "OverrideRootScale" null null))
  (`KismetArrayLibrary.Array_Add` _robotalive _returnvalue_3)
  ;[1 1 1] Spawning robot 4
  (bind _randomtransform_4 (`self.Random Transform`))
  (bind _returnvalue_4 (`|SpawnActorFromClass` "/Game/Blueprint/RobotTest_BP.RobotTest_BP_C" _randomtransform_4 "Undefined" "OverrideRootScale" null null))
  (`KismetArrayLibrary.Array_Add` _robotalive _returnvalue_4)
  ;[1 1 1] Set Robots Color
  (for (_array_element _array_index) _robotalive
    (`Robot.SetRobotColor` _array_element (`|GetArrayItem` (`self.ColorArray`) _array_index))
    ;[1 1 1] Create the UI for each Robot
    (bind _returnvalue_5 (`|CreateWidget` "/Game/Widget/MainWidget_BP.MainWidget_BP_C"))
    (`UserWidget.AddToViewport` _returnvalue_5 0)
    (`WidgetBlueprintLibrary.SetInputMode_UIOnlyEx` (`GameplayStatics.GetPlayerController` 0) _returnvalue_5)))

(event `self.ReceiveTick`
  (params (DeltaSeconds :type "Float (single-precision)")))

(fn `Random Transform`
  (returns (RandomTransform :type "Transform Structure"))
  (bind _maxarenaesize (`self.MaxArenaeSize`))
  (bind _minarenasize (`self.MinArenaSize`))
  (return (`KismetMathLibrary.MakeTransform` (`KismetMathLibrary.MakeVector` (`KismetMathLibrary.RandomFloatInRange` _minarenasize _maxarenaesize) (`KismetMathLibrary.RandomFloatInRange` _minarenasize _maxarenaesize) 40.0) (`KismetMathLibrary.MakeRotator` 0.0 0.0 (`KismetMathLibrary.RandomFloatInRange` 0.0 360.0)))))

(fn `Randomise Robot`
  (for _array_element (`self.RobotAlive`)
    (bind _randomtransform (`self.Random Transform`))
    (`self.K2_SetActorRotation` _array_element (.rotation _randomtransform) false)
    (`SceneComponent.K2_SetWorldLocation` (`Actor.RootComponent` _array_element) (.location _randomtransform) false false)
    (return)))

(fn `UserConstructionScript`)